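; BulletBP is a bullet actor that damages actors tagged "enemy" using the player's shot damage.
; On BeginPlay it finds the first PlayerCharacterBP in the level and caches it as Player.
; When Sphere1 begins overlapping a tagged actor, it applies the player's current Shootdamage, converted to float, then destroys itself.
; Overlaps with untagged actors are ignored, and the graph contains no movement logic.
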(event OnComponentBeginOverlap(Sphere1)
  (params (OverlappedComponent :type Primitive%20Component%20Object%20Reference) (OtherActor :type Actor%20Object%20Reference) (OtherComp :type Primitive%20Component%20Object%20Reference) (OtherBodyIndex :type Integer) (bFromSweep :type Boolean) (SweepResult :type Hit%20Result%20Structure%20%28by%20ref%29))
  (if (Actor|ActorHasTag OtherActor "enemy")
    (Game|Damage|ApplyDamage OtherActor (Math|Conversions|ToFloat(Integer) (Variables|/Script/ZadanieTestowe.PlayerCharacterCpp|Getshootdamage (Variables|Default|GetPlayer))) 0 0)
    (Actor|DestroyActor)))

(event EventBeginPlay
  (bind _outactors (Actor|GetAllActorsOfClass "/Game/Player/PlayerCharacterBP.PlayerCharacterBP_C"))
  (bind _asplayer_character_bp (Utilities|Casting|CastToPlayerCharacterBP (Utilities|Array|Get(acopy) _outactors)))
  (Variables|Default|SetPlayer _asplayer_character_bp))

(event Collision|EventActorBeginOverlap
  (params (OtherActor :type Actor%20Object%20Reference)))

(event EventTick
  (params (DeltaSeconds :type Float%20%28single-precision%29)))

(fn ConstructionScript)