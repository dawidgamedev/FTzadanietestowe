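; Player character Blueprint that automatically pursues and shoots at enemies.
; While movement is allowed, Tick scans all EnemyBP actors for the nearest, using a stored minimum distance that is never reset here.
; If that enemy is within Shootdistance, the character navigates toward it with SimpleMoveToActor and turns to face it.
; When PlayerCanShoot is set, it calls ShootFunction from Arrow1's transform and plays a sound.
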(event EventTick
  (params (DeltaSeconds :type Float%20%28single-precision%29))
  (bind _nearestenemy (Variables|Default|GetNearestEnemy))
  (bind _arrow1 (Variables|Default|GetArrow1))
  (if (Variables|Default|GetCanMovement)
    (CallFunction|GetNearestEnemy)
    (Utilities|IsValid _nearestenemy
      (:Is%20Valid
        (if (< (Math|Vector|Distance(Vector) (Transformation|GetActorLocation _nearestenemy) (Transformation|GetActorLocation)) (Math|Conversions|ToFloat(Integer) (Variables|Default|Getshootdistance)))
          (AI|Navigation|SimpleMovetoActor (Game|GetPlayerController 0) _nearestenemy)
          (CallFunction|SetRotationtoEnemy)
          (if (Variables|Default|GetbPlayerCanShoot)
            (Class|PlayerCharacterCpp|ShootFunction (Transformation|GetWorldLocation _arrow1) (Transformation|GetWorldRotation _arrow1))
            (Audio|PlaySound2D "/Game/Player/ShootSound.ShootSound" 1.0 1.0 0.0 0 0)))))))

(fn ConstructionScript)

(fn GetNearestEnemy
  (bind _outactors (Actor|GetAllActorsOfClass "/Game/Enemy/EnemyBP.EnemyBP_C"))
  (for _array_element _outactors
    (if (< (Math|Vector|Distance(Vector) (Transformation|GetActorLocation _array_element) (Transformation|GetActorLocation)) (Variables|Default|GetNearestEnemyDistance))
      (Variables|Default|SetNearestEnemyDistance (Math|Vector|Distance(Vector) (Transformation|GetActorLocation _array_element) (Transformation|GetActorLocation)))
      (Variables|Default|SetNearestEnemy _array_element))))

(fn SetRotationtoEnemy
  (Transformation|SetActorRotation (Math|Rotator|FindLookatRotation (Transformation|GetActorLocation) (Transformation|GetActorLocation (Variables|Default|GetNearestEnemy)))))